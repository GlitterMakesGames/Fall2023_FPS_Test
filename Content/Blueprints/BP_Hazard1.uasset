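; BP_Hazard1 is a moving hazard actor that loops endlessly through a list of node actors.
; Each Tick it lerps a fixed fraction of the way toward the current node's location without sweeping, so it eases in as it nears each point.
; Once within a small distance it advances the node index, wrapping back to the first.
; The file contains no damage or overlap logic.
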(event EventBeginPlay)

(event Collision|EventActorBeginOverlap
  (params (OtherActor :type Actor%20Object%20Reference)))

(event EventTick
  (params (DeltaSeconds :type Float%20%28single-precision%29))
  (bind _returnvalue (Transformation|GetActorLocation))
  (Transformation|SetActorLocation (Math|Vector|Lerp(Vector) _returnvalue (Transformation|GetWorldLocation (Variables|/Script/Engine.Actor|GetRootComponent (Utilities|Array|Get(acopy) (Variables|Default|Getnodes) (Variables|Default|GetnodeIndex)))) 0.05) false false)
  (if (<= (Math|Vector|Distance(Vector) _returnvalue (Transformation|GetWorldLocation (Variables|/Script/Engine.Actor|GetRootComponent (Utilities|Array|Get(acopy) (Variables|Default|Getnodes) (Variables|Default|GetnodeIndex))))) 1.0)
    (Math|Integer|IncrementInt (Variables|Default|GetnodeIndex)
      (:%20%20
        (if (>= (Variables|Default|GetnodeIndex) (Utilities|Array|Length (Variables|Default|Getnodes)))
          (Variables|Default|SetnodeIndex 0))))))

(fn ConstructionScript)